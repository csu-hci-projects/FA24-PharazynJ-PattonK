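; BP_Barrel is a barrel that catches fire when shot and burns the nearby player.
; A hit from BP_FirstPersonProjectile sets OnFire and unhides the fire particle effect.
; While burning, Tick runs through a one-second Delay, throttling damage checks to roughly once per second.
; Each check applies damage to the first player's character if it overlaps DamageRadius, and nothing puts the fire out.
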(event EventTick
  (params (DeltaSeconds :type Float%20%28single-precision%29))
  (bind _returnvalue (Game|GetPlayerCharacter 0))
  (if (Variables|Default|GetOnFire)
    (Utilities|FlowControl|Delay 1.0)
    (if (Collision|IsOverlappingActor (Variables|Default|GetDamageRadius) _returnvalue :!class /Script/Engine.PrimitiveComponent)
      (Game|Damage|ApplyDamage _returnvalue 1e+01 0 self "/Script/Engine.DamageType"))))

(event Collision|EventHit
  (params (MyComp :type Primitive%20Component%20Object%20Reference) (Other :type Actor%20Object%20Reference) (OtherComp :type Primitive%20Component%20Object%20Reference) (bSelfMoved :type Boolean) (HitLocation :type Vector :default "0, 0, 0") (HitNormal :type Vector :default "0, 0, 0") (NormalImpulse :type Vector :default "0, 0, 0") (Hit :type Hit%20Result%20Structure%20%28by%20ref%29))
  (Utilities|Casting|CastToBP_FirstPersonProjectile Other)
  (Variables|Default|SetOnFire true)
  (Development|SetHiddeninGame (Variables|/Game/StarterContent/Blueprints/Blueprint_Effect_Fire.Blueprint_Effect_Fire_C|GetP_Fire (Variables|Default|GetFireEffect)) false false))

(fn ConstructionScript)